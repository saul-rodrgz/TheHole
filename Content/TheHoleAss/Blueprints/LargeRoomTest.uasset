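; LargeRoomTest is a test room actor that chains copies of itself as the player advances, apparently prototyping procedural room generation.
; A looping timer polls the player character's distance to the DoorEnd component, printing debug text until a room spawns.
; Within range, it spawns another LargeRoomTest at a fixed offset in DoorEnd's local space, adjusting for or aborting on collision.
; It then sets a one-shot flag and destroys DoorEnd.
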(event Custom|CheckDistanceToPlayer
  (if (Math|Boolean|Equal(Boolean) (Variables|Default|GetRoomSpawned) false)
    (Variables|Default|SetVectorDistToPlayer (Math|Vector|VectorLength (- (Transformation|GetActorLocation (Game|GetPlayerCharacter 0)) (Transformation|GetWorldLocation (Variables|Default|GetDoorEnd)))))
    (if (<= (Variables|Default|GetVectorDistToPlayer) 1.9e+02)
      (Development|PrintString "INSIDE DISTANCE" true true "(R=0.095608,G=1.000000,B=0.137434,A=1.000000)")
      (Development|PrintString (Utilities|String|ToString(Float) (Variables|Default|GetVectorDistToPlayer)))
      (Game|SpawnActorfromClass "LargeRoomTest_C" (Math|Conversions|ToTransform(Vector) (Math|Transform|TransformLocation (Transformation|GetWorldTransform (Variables|Default|GetDoorEnd)) "1620.000000,-40.000000,20.000000")) "AdjustIfPossibleButDontSpawnIfColliding" 0 0)
      (Variables|Default|SetRoomSpawned true)
      (Components|DestroyComponent (Variables|Default|GetDoorEnd))
      (else
        (Development|PrintString "Outside DISTANCE" true true "(R=1.000000,G=0.030093,B=0.010197,A=1.000000)")
        (Development|PrintString (Utilities|String|ToString(Float) (Variables|Default|GetVectorDistToPlayer)))))))

(event Collision|EventActorBeginOverlap
  (params (OtherActor :type Actor%20Object%20Reference)))

(event EventTick
  (params (DeltaSeconds :type Float%20%28single-precision%29)))

(event EventBeginPlay
  (Utilities|Time|SetTimerbyFunctionName 0 "CheckDistanceToPlayer" 0.5 true))

(fn ConstructionScript)