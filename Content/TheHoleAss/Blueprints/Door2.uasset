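; Door actor Blueprint that turns its Cube into a physics object shortly after play begins.
; BeginPlay waits a few seconds, then calls TurnOnPhysics, which enables simulation on the Cube and sets the PointLight to high intensity.
; The same event also issues an attach of the Cube's owner to the PointLight, keeping relative transforms.
; Spawn and print snippets are unconnected, and the overlap and tick events are disabled.
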(event Custom|TurnOnPhysics
  (Physics|SetSimulatePhysics (Variables|Default|GetCube) true)
  (Rendering|Components|Light|SetIntensity (Variables|Default|GetPointLight) 1e+04)
  (Transformation|AttachComponentToComponent (Components|GetOwner (Variables|Default|GetCube)) (Variables|Default|GetPointLight) "None" "KeepRelative" "KeepRelative" "KeepRelative" true))

(event EventBeginPlay
  (Utilities|FlowControl|Delay 3.0)
  (CallFunction|TurnonPhysics))

(event Collision|EventActorBeginOverlap
  (params (OtherActor :type Actor%20Object%20Reference)))

(event EventTick
  (params (DeltaSeconds :type Float%20%28single-precision%29)))

(fn ConstructionScript)