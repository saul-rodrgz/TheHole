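; SmallRoomTest is a test room actor with four trigger boxes (N, S, E, W) that prompt the first-person character to interact.
; Each box's overlap creates a prompt widget and opens its own Gate; leaving removes the widget and closes it.
; The Interact input feeds all four gates, but none has an output action wired.
; The east box's CreateWidget has no class set, and its end overlap prints the widget's name.
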(event OnComponentBeginOverlap(BoxN)
  (params (OverlappedComponent :type Primitive%20Component%20Object%20Reference) (OtherActor :type Actor%20Object%20Reference) (OtherComp :type Primitive%20Component%20Object%20Reference) (OtherBodyIndex :type Integer) (bFromSweep :type Boolean) (SweepResult :type Hit%20Result%20Structure%20%28by%20ref%29))
  ;[1 1 1] Checks if we are close enough
  (Utilities|Casting|CastToFirstPersonCharacter OtherActor)
  ;[1 1 1] Add and remove prompt from screen
  (bind _returnvalue (UserInterface|CreateWidget "/Game/TheHoleAss/Blueprints/InteractPromptWidget.InteractPromptWidget_C"))
  (UserInterface|Viewport|AddtoViewport _returnvalue 0)
  (Utilities|FlowControl|Gate true) ; enters at Open
)

(event OnComponentEndOverlap(BoxN)
  (params (OverlappedComponent :type Primitive%20Component%20Object%20Reference) (OtherActor :type Actor%20Object%20Reference) (OtherComp :type Primitive%20Component%20Object%20Reference) (OtherBodyIndex :type Integer))
  ;[1 1 1] Checks if we are close enough
  (Utilities|Casting|CastToFirstPersonCharacter OtherActor)
  ;[1 1 1] Add and remove prompt from screen
  (Widget|RemovefromParent (stale OnComponentBeginOverlap(BoxN) _returnvalue))
  (Utilities|FlowControl|Gate true) ; enters at Close
)

(event OnComponentBeginOverlap(BoxS)
  (params (OverlappedComponent :type Primitive%20Component%20Object%20Reference) (OtherActor :type Actor%20Object%20Reference) (OtherComp :type Primitive%20Component%20Object%20Reference) (OtherBodyIndex :type Integer) (bFromSweep :type Boolean) (SweepResult :type Hit%20Result%20Structure%20%28by%20ref%29))
  ;[1 1 1] Checks if we are close enough
  (Utilities|Casting|CastToFirstPersonCharacter OtherActor)
  ;[1 1 1] Add and remove prompt from screen
  (bind _returnvalue (UserInterface|CreateWidget "/Game/TheHoleAss/Blueprints/InteractPromptWidget.InteractPromptWidget_C"))
  (UserInterface|Viewport|AddtoViewport _returnvalue 0)
  (Utilities|FlowControl|Gate true) ; enters at Open
)

(event OnComponentEndOverlap(BoxS)
  (params (OverlappedComponent :type Primitive%20Component%20Object%20Reference) (OtherActor :type Actor%20Object%20Reference) (OtherComp :type Primitive%20Component%20Object%20Reference) (OtherBodyIndex :type Integer))
  ;[1 1 1] Checks if we are close enough
  (Utilities|Casting|CastToFirstPersonCharacter OtherActor)
  ;[1 1 1] Add and remove prompt from screen
  (Widget|RemovefromParent (stale OnComponentBeginOverlap(BoxS) _returnvalue))
  (Utilities|FlowControl|Gate true) ; enters at Close
)

(event OnComponentBeginOverlap(BoxW)
  (params (OverlappedComponent :type Primitive%20Component%20Object%20Reference) (OtherActor :type Actor%20Object%20Reference) (OtherComp :type Primitive%20Component%20Object%20Reference) (OtherBodyIndex :type Integer) (bFromSweep :type Boolean) (SweepResult :type Hit%20Result%20Structure%20%28by%20ref%29))
  ;[1 1 1] Checks if we are close enough
  (Utilities|Casting|CastToFirstPersonCharacter OtherActor)
  ;[1 1 1] Add and remove prompt from screen
  (bind _returnvalue (UserInterface|CreateWidget "/Game/TheHoleAss/Blueprints/InteractPromptWidget.InteractPromptWidget_C"))
  (UserInterface|Viewport|AddtoViewport _returnvalue 0)
  (Utilities|FlowControl|Gate true) ; enters at Open
)

(event OnComponentEndOverlap(BoxW)
  (params (OverlappedComponent :type Primitive%20Component%20Object%20Reference) (OtherActor :type Actor%20Object%20Reference) (OtherComp :type Primitive%20Component%20Object%20Reference) (OtherBodyIndex :type Integer))
  ;[1 1 1] Checks if we are close enough
  (Utilities|Casting|CastToFirstPersonCharacter OtherActor)
  ;[1 1 1] Add and remove prompt from screen
  (Widget|RemovefromParent (stale OnComponentBeginOverlap(BoxW) _returnvalue))
  (Utilities|FlowControl|Gate true) ; enters at Close
)

(event OnComponentBeginOverlap(BoxE)
  (params (OverlappedComponent :type Primitive%20Component%20Object%20Reference) (OtherActor :type Actor%20Object%20Reference) (OtherComp :type Primitive%20Component%20Object%20Reference) (OtherBodyIndex :type Integer) (bFromSweep :type Boolean) (SweepResult :type Hit%20Result%20Structure%20%28by%20ref%29))
  ;[1 1 1] Checks if we are close enough
  (Utilities|Casting|CastToFirstPersonCharacter OtherActor)
  ;[1 1 1] Add and remove prompt from screen
  (bind _returnvalue (UserInterface|CreateWidget "/Game/TheHoleAss/Blueprints/InteractPromptWidget.InteractPromptWidget_C"))
  (UserInterface|Viewport|AddtoViewport _returnvalue 0)
  (Utilities|FlowControl|Gate true) ; enters at Open
)

(event OnComponentEndOverlap(BoxE)
  (params (OverlappedComponent :type Primitive%20Component%20Object%20Reference) (OtherActor :type Actor%20Object%20Reference) (OtherComp :type Primitive%20Component%20Object%20Reference) (OtherBodyIndex :type Integer))
  ;[1 1 1] Checks if we are close enough
  (Utilities|Casting|CastToFirstPersonCharacter OtherActor)
  ;[1 1 1] Add and remove prompt from screen
  (Widget|RemovefromParent (stale OnComponentBeginOverlap(BoxE) _returnvalue))
  (Development|PrintString (Utilities|GetDisplayName (stale OnComponentBeginOverlap(BoxE) _returnvalue)))
  (Utilities|FlowControl|Gate true) ; enters at Close
)

(event EventBeginPlay)

(event Collision|EventActorBeginOverlap
  (params (OtherActor :type Actor%20Object%20Reference)))

(event EventTick
  (params (DeltaSeconds :type Float%20%28single-precision%29)))

(event Input|ActionEvents|InputActionInteract
  (params (Key :type Key%20Structure :default "None"))
  (:Pressed
    (Utilities|FlowControl|Gate true)))

(event Input|ActionEvents|InputActionInteract
  (params (Key :type Key%20Structure :default "None"))
  (:Pressed
    (Utilities|FlowControl|Gate true)))

(event Input|ActionEvents|InputActionInteract
  (params (Key :type Key%20Structure :default "None"))
  (:Pressed
    (Utilities|FlowControl|Gate true)))

(event Input|ActionEvents|InputActionInteract
  (params (Key :type Key%20Structure :default "None"))
  (:Pressed
    (Utilities|FlowControl|Gate true)))

(fn ConstructionScript)